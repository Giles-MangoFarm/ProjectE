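; Enemy guard that patrols a looping four-point path with random waits and a visible line-of-sight mesh built from traces.
; Seeing a pawn starts its detection message, cleared by a retriggerable delay after sight stops, which also resumes patrol.
; Custom events toggle ShouldChase, which makes sightings trigger a faster chase of the player.
; When not chasing, perception stimuli send the guard to investigate their location before returning to patrol.
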(event `self.ReceiveBeginPlay`
  (bind _lineofsight (`self.LineOfSight`))
  ;[1 1 1] Create Line of Sight
  (`LineOfSightComponent.StartLineTrace` _lineofsight "TraceTypeQuery1" 60)
  (`LineOfSightComponent.StartBuildMesh` _lineofsight)
  (`self.GuardPatrol` "Called on CreateLOS"))

(event `self.PawnSensing.OnSeePawn`
  (params (Pawn :type "Pawn Object Reference"))
  (bind _charactermovement (`self.CharacterMovement`))
  ;[1 1 1] Detection/Chase
  (`|ExecutionSequence`
    (:`then_0`
      (`|ExecutionSequence`
        (:`then_0`
          (`/Engine/EditorBlueprintResources/StandardMacros.DoOnce` false :!label _label
            (:`Completed`
              (message `/Game/ThirdPerson/Blueprints/BP_DetectionInterface.StartDetection` Pawn self))))
        (:`then_1`
          (if (`self.ShouldChase`)
            (set `CharacterMovementComponent.MaxWalkSpeed` 401.0 _charactermovement)
            (`|AIMoveTo` (`CharacterMovementComponent.GetCharacterOwner` _charactermovement) (0.0 0.0 0.0) (`GameplayStatics.GetPlayerPawn` 0))))))
    (:`then_1`
      (`KismetSystemLibrary.RetriggerableDelay` 0.5)
      (message `/Game/ThirdPerson/Blueprints/BP_DetectionInterface.StopDetection` Pawn)
      (`self.GuardPatrol` "Called after StopDetection")
      (goto _label :!via `Reset`))))

(event `CustomEvent`
  ;[1 1 1] Detection/Chase
  (set `self.ShouldChase` true))

(event `CustomEvent_1`
  ;[1 1 1] Detection/Chase
  (set `self.ShouldChase` false)
  (`|AIMoveTo` self (0.0 0.0 0.0) self ; Makes NPC stop chasing
    (:`then`
      (`self.GuardPatrol` "Called from StopChase"))))

(event `self.AIPerception.OnTargetPerceptionUpdated`
  (params (Actor :type "Actor Object Reference") (Stimulus :type "AIStimulus Structure"))
  ;[1 1 1] Sound Investigation
  (if (not (`self.ShouldChase`))
    (`|AIMoveTo` (`CharacterMovementComponent.GetCharacterOwner` (`self.CharacterMovement`)) Stimulus_StimulusLocation null
      (:`OnSuccess`
        (`KismetSystemLibrary.Delay` 3.0)
        (`self.GuardPatrol` "Called from SoundInvestigation")))))

(event `GuardPatrol`
  (params (DebugLog :type String))
  ;[1 1 1] Patrol
  (`KismetSystemLibrary.PrintString` DebugLog true true (struct :`G` 0.66 :`B` 1.0 :`A` 1.0) 12.0)
  (set `CharacterMovementComponent.MaxWalkSpeed` 200.0 (`self.CharacterMovement`))
  (`|AIMoveTo` self (`|GetArrayItem` (`self.PatrolPath`) (`self.PatrolIndex`)) null
    (:`OnSuccess`
      (`KismetSystemLibrary.Delay` (`KismetMathLibrary.RandomFloatInRange` 2.0 5.0))
      (`/Engine/EditorBlueprintResources/StandardMacros.IncrementInt` (`self.PatrolIndex`)
        (:`  `
          (if (== (`self.PatrolIndex`) 4)
            (set `self.PatrolIndex` 0))
          (`self.GuardPatrol` "Called in Patrol"))))))

(fn `UserConstructionScript`)