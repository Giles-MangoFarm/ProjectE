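; Enemy guard character that spots, chases and investigates noises, with a line-of-sight mesh built from traces at BeginPlay.
; PawnSensing notifies the seen pawn once, clearing the message after sightings lapse via a retriggerable delay, and chases the player while ShouldChase is set.
; StartChase and StopChase toggle that flag.
; When not chasing, AIPerception stimuli draw it to their location, then GuardPatrol lowers speed and issues a move with no destination set.
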(event `self.ReceiveBeginPlay`
  (bind _lineofsight (`self.LineOfSight`))
  ;[1 1 1] Create Line of Sight
  (`LineOfSightComponent.StartLineTrace` _lineofsight "TraceTypeQuery1" 60)
  (`LineOfSightComponent.StartBuildMesh` _lineofsight))

(event `self.PawnSensing.OnSeePawn`
  (params (Pawn :type "Pawn Object Reference"))
  (bind _charactermovement (`self.CharacterMovement`))
  ;[1 1 1] Detection/Chase
  (`|ExecutionSequence`
    (:`then_0`
      (`|ExecutionSequence`
        (:`then_0`
          (`/Engine/EditorBlueprintResources/StandardMacros.DoOnce` false :!label _label
            (:`Completed`
              (message `/Game/ThirdPerson/Blueprints/BP_DetectionInterface.StartDetection` Pawn self))))
        (:`then_1`
          (if (`self.ShouldChase`)
            (set `CharacterMovementComponent.MaxWalkSpeed` 401.0 _charactermovement)
            (`|AIMoveTo` (`CharacterMovementComponent.GetCharacterOwner` _charactermovement) (0.0 0.0 0.0) (`GameplayStatics.GetPlayerPawn` 0))))))
    (:`then_1`
      (`KismetSystemLibrary.RetriggerableDelay` 0.5)
      (message `/Game/ThirdPerson/Blueprints/BP_DetectionInterface.StopDetection` Pawn)
      (goto _label :!via `Reset`))))

(event `/Game/ThirdPerson/Blueprints/BP_DetectionInterface.StartChase`
  ;[1 1 1] Detection/Chase
  (set `self.ShouldChase` true))

(event `/Game/ThirdPerson/Blueprints/BP_DetectionInterface.StopChase`
  ;[1 1 1] Detection/Chase
  (set `self.ShouldChase` false)
  (`|AIMoveTo` self (0.0 0.0 0.0) self))

(event `self.AIPerception.OnTargetPerceptionUpdated`
  (params (Actor :type "Actor Object Reference") (Stimulus :type "AIStimulus Structure"))
  ;[1 1 1] Sound Investigation
  (if (not (`self.ShouldChase`))
    (`|AIMoveTo` (`CharacterMovementComponent.GetCharacterOwner` (`self.CharacterMovement`)) Stimulus_StimulusLocation null
      (:`OnSuccess`
        (`KismetSystemLibrary.Delay` 0.2)
        (`self.GuardPatrol`)))))

(event `GuardPatrol`
  (set `CharacterMovementComponent.MaxWalkSpeed` 200.0 (`self.CharacterMovement`))
  (`|AIMoveTo` null (0.0 0.0 0.0) null))

(fn `UserConstructionScript`)